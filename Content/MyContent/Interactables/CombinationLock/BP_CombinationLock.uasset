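; BP_CombinationLock is an interactable chest with a combination lock that yields an item when unlocked.
; On BeginPlay it creates a W_CombinationLockUI widget, gives it the combination and a self reference, then hands it to its combination lock component.
; Overlap reports it as interactable with an open prompt, while Interactwith is empty here.
; Unlock spawns the Item at the chest's transform, plays a lock sound and destroys the chest.
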(event `self.InteractWith`
  (params (Player :type "/Game/TopDown/Blueprints/BP_TopDownCharacter Object Reference")))

(event `self.ReceiveBeginPlay`
  (bind _returnvalue (`|CreateWidget` "/Game/MyContent/Interactables/UI/W_CombinationLockUI.W_CombinationLockUI_C"))
  (bind _output_get (set `self.Menu` _returnvalue))
  (`/Game/MyContent/Interactables/UI/W_CombinationLockUI.setCombination` _output_get (`self.Combination`))
  (`/Game/MyContent/Interactables/UI/W_CombinationLockUI.setChest` _output_get self)
  (`/Game/MyContent/Interactables/CombinationLock/BP_CombinationLockCompoment.SetMenu` (`self.BP_CombinationLockCompoment`) (`self.Menu`)))

(fn `Overlap`
  (returns (interactable :type Boolean) (text :type Text))
  (return true "Press E to open the chest "))

(fn `unlock`
  (`|SpawnActorFromClass` (`self.Item`) (`self.GetTransform`) "Undefined" "MultiplyWithRoot" null null)
  (`GameplayStatics.PlaySound2D` "/Game/MyContent/Sounds/lock-sound-effect-247455.lock-sound-effect-247455" 1.0 1.0 0.0 null null)
  (`self.K2_DestroyActor`))

(fn `UserConstructionScript`)