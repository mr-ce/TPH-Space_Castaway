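; BP_Book is an interactable book that offers a "Press E to open the book" prompt when overlapped.
; On BeginPlay it creates a W_TextUI widget, fills its left and right text from TextLeft and TextRight, and passes it to BPBookCompoment as its menu.
; Its own Interactwith event is empty.
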(event `/Game/MyContent/Interactables/I_InteractInterface.InteractWith`
  (params (Player :type "/Game/TopDown/Blueprints/BP_TopDownCharacter Object Reference")))

(event `self.ReceiveBeginPlay`
  (bind _returnvalue (`|CreateWidget` "/Game/MyContent/Interactables/UI/W_TextUI.W_TextUI_C"))
  (bind _output_get (set `self.Menu` _returnvalue))
  (`/Game/MyContent/Interactables/UI/W_TextUI.SetTextLeft` _output_get (`self.textLeft`))
  (`/Game/MyContent/Interactables/UI/W_TextUI.SetTextRight` _output_get (`self.textRight`))
  (`/Game/MyContent/Interactables/Book/BP_BookCompoment.SetMenu` (`self.BP_BookCompoment`) (`self.Menu`)))

(fn `Overlap`
  (returns (interactable :type Boolean) (text :type Text))
  (return true "Press E to open the book "))

(fn `UserConstructionScript`)