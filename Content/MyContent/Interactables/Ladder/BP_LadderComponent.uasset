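; BP_LadderComponent is an interaction component that lets the player spend items, apparently planks, to activate its owning actor, presumably a ladder.
; Interactwith removes the configured item and quantity from the player's InventorySystem, then plays a wood sound, messages the owner and sets Activated, making it one-shot.
; On failed removal it shows a hardcoded plank-requirement message through the top-down character cached at BeginPlay.
; Overlap reports it interactable until activated, with placeholder prompt text.
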(event `/Game/MyContent/Interactables/I_InteractInterface.InteractWith`
  (params (Player :type "/Game/TopDown/Blueprints/BP_TopDownCharacter Object Reference"))
  (bind _inventorysystem (`/Game/TopDown/Blueprints/BP_TopDownCharacter.InventorySystem` Player))
  (bind (_itemid_datatable _itemid_rowname) (break `DataTableRowHandle` (`self.ItemID`)))
  (if (not (`self.Activated`))
    (`/Engine/EditorBlueprintResources/StandardMacros.IsValid` _inventorysystem
      (:`Is Valid`
        (bind _success (`/Game/MyContent/Inventory/InventorySystem.RemoveFromInventory` _inventorysystem _itemid_rowname (`self.Quantity`)))
        (if _success
          (`GameplayStatics.PlaySound2D` "/Game/MyContent/Sounds/impact_wood_planks_x2_drop_on_floor_together_001.impact_wood_planks_x2_drop_on_floor_together_001" 1.0 1.0 0.0 null null)
          (message `/Game/MyContent/Interactables/I_InteractInterface.InteractWith` (`self.GetOwner`) null)
          (set `self.Activated` true)
          (else
            (`/Game/TopDown/Blueprints/BP_TopDownCharacter.SetUIText` (stale `self.ReceiveBeginPlay` _output_get) "You need 16 planks")))))))

(event `self.ReceiveBeginPlay`
  (bind _asbp_top_down_character (cast `/Game/TopDown/Blueprints/BP_TopDownCharacter` (`GameplayStatics.GetPlayerPawn` 0)))
  (bind _output_get (set `self.Character` _asbp_top_down_character)))

(fn `Overlap`
  (returns (interactable :type Boolean) (text :type Text))
  (return (not (`self.Activated`)) "dasdasd"))