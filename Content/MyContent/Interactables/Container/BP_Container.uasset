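; BP_Container is an interactable container that is replaced by a spawned item when unlocked.
; On BeginPlay it hands itself and its NeededItem to BPContainerCompoment, while the construction script applies the configurable Model mesh.
; Overlap returns a "Press E to" prompt, but Interactwith is empty.
; Unlock plays a 2D sound, spawns Item at the container's transform and destroys the container.
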(event `self.ReceiveBeginPlay`
  (bind _bp_containercompoment (`self.BP_ContainerCompoment`))
  (`/Game/MyContent/Interactables/Container/BP_ContainerCompoment.SetContainer` _bp_containercompoment self)
  (`/Game/MyContent/Interactables/Container/BP_ContainerCompoment.SetNeededItem` _bp_containercompoment (`self.NeededItem`)))

(event `/Game/MyContent/Interactables/I_InteractInterface.InteractWith`
  (params (Player :type "/Game/TopDown/Blueprints/BP_TopDownCharacter Object Reference")))

(fn `Overlap`
  (returns (interactable :type Boolean) (text :type Text))
  (return true (`|FormatText` "Press E to {0}" (`self.Text`))))

(fn `unlock`
  (`GameplayStatics.PlaySound2D` (`self.Sound`) 1.0 1.0 0.0 null null)
  (`|SpawnActorFromClass` (`self.Item`) (`self.GetTransform`) "Undefined" "MultiplyWithRoot" null null)
  (`self.K2_DestroyActor`))

(fn `UserConstructionScript`
  (`StaticMeshComponent.SetStaticMesh` (`self.Pivot`) (`self.Model`)))