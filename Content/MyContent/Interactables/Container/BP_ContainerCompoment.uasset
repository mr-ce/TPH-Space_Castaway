(event `self.InteractWith`
  (params (Player :type "/Game/TopDown/Blueprints/BP_TopDownCharacter Object Reference"))
  (bind _inventorysystem (`/Game/TopDown/Blueprints/BP_TopDownCharacter.InventorySystem` Player))
  (if (== (`self.ItemID`) "None")
    (`/Game/MyContent/Interactables/Container/BP_Container.unlock` (`self.Container`) :!label _label)
    (else
      (`/Engine/EditorBlueprintResources/StandardMacros.IsValid` _inventorysystem
        (:`Is Valid`
          (bind (_index _foundslot) (`/Game/MyContent/Inventory/InventorySystem.Find Item` _inventorysystem (`self.ItemID`)))
          (if _foundslot
            (goto _label)
            (else
              (`/Game/TopDown/Blueprints/BP_TopDownCharacter.SetUIText` (stale `self.ReceiveBeginPlay` _output_get) (`|FormatText` "You need a {0}" (`KismetTextLibrary.Conv_NameToText` (`self.ItemID`)))))))))))

(event `self.ReceiveBeginPlay`
  (bind _asbp_top_down_character (cast `/Game/TopDown/Blueprints/BP_TopDownCharacter` (`GameplayStatics.GetPlayerPawn` 0)))
  (bind _output_get (set `self.Character` _asbp_top_down_character)))

(fn `Overlap`
  (returns (interactable :type Boolean) (text :type Text))
  (return true "Press E to open the book"))

(fn `SetContainer`
  (params (container :type "/Game/MyContent/Interactables/Container/BP_Container Object Reference"))
  (set `self.Container` container))

(fn `SetNeededItem`
  (params (NeededItem :type Name))
  (set `self.ItemID` NeededItem))